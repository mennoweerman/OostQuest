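; BP_LocationManager starts mobile GPS location services and shows the device's coordinates as on-screen debug text.
; BeginPlay initializes navigation-accuracy tracking, prints the init and start results, and binds to the location-changed delegate.
; Each update is stored as a longitude-latitude string, flagged in red when it differs from the previous one and printed persistently under a key.
; Tick separately polls and prints the last known location for comparison.
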(event `self.ReceiveBeginPlay`
  (bind _returnvalue (`LocationServices.InitLocationServices` "LA_Navigation" 1000.0 1e-06))
  (`KismetSystemLibrary.PrintString` (`KismetStringLibrary.Conv_BoolToString` _returnvalue))
  (bind _returnvalue_2 (`LocationServices.StartLocationServices`))
  (`KismetSystemLibrary.PrintString` (`KismetStringLibrary.Conv_BoolToString` _returnvalue_2))
  (bind _returnvalue_3 (`LocationServices.GetLocationServicesImpl`))
  (add `LocationServicesImpl.OnLocationChanged` _returnvalue_3 (delegate `OnLocationChanged_Event`)))

(event `OnLocationChanged_Event`
  (params (LocationData :type "LocationServicesData Structure"))
  (bind _returnvalue (`KismetStringLibrary.Concat_StrStr` (`KismetStringLibrary.Conv_DoubleToString` LocationData_Longitude) " - " (`KismetStringLibrary.Conv_DoubleToString` LocationData_Latitude)))
  (if (not (== (`self.NewVar`) _returnvalue))
    (`KismetSystemLibrary.PrintString` "NEW LOCATION" true true (struct :`R` 1.0 :`A` 1.0)))
  (bind _output_get (set `self.NewVar` _returnvalue))
  (`KismetSystemLibrary.PrintString` (`KismetStringLibrary.Concat_StrStr` _output_get " - " "Last known location update") true true (struct :`G` 0.66 :`B` 1.0 :`A` 1.0) 2e+19 "LocationPrint"))

(event `self.ReceiveTick`
  (params (DeltaSeconds :type "Float (single-precision)"))
  (bind _returnvalue (`LocationServices.GetLastKnownLocation`))
  (`KismetSystemLibrary.PrintString` (`KismetStringLibrary.Concat_StrStr` (`KismetStringLibrary.Conv_DoubleToString` (`.Longitude` (break `LocationServicesData` _returnvalue))) " - " (`KismetStringLibrary.Conv_DoubleToString` (`.Latitude` (break `LocationServicesData` _returnvalue)))) true true (struct :`G` 0.66 :`B` 1.0 :`A` 1.0) 2.0 "LastKnownLocation"))

(fn `UserConstructionScript`)